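; BP_PressureButton is a pressure button that holds a linked Door open while something overlaps its TriggerBox.
; Begin and end overlap events add and remove actors in OverlappingActors, with no filtering by actor type.
; The button sets IsPressed and calls OpenDoor on each new overlap, then clears it and calls CloseDoor once the array empties.
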(event `self.TriggerBox.OnComponentBeginOverlap`
  (params (OverlappedComponent :type "PrimitiveComponent Object Reference") (OtherActor :type "Actor Object Reference") (OtherComp :type "PrimitiveComponent Object Reference") (OtherBodyIndex :type Integer) (bFromSweep :type Boolean) (SweepResult :type "HitResult Structure (by ref)"))
  (bind _overlappingactors (`self.OverlappingActors`))
  (`KismetArrayLibrary.Array_Add` _overlappingactors OtherActor)
  (if (> (`KismetArrayLibrary.Array_Length` _overlappingactors) 0)
    (set `self.bIsPressed` true)
    (`/Game/_Main/Blueprints/Object/BP_Door.OpenDoor` (`self.Door`))))

(event `self.TriggerBox.OnComponentEndOverlap`
  (params (OverlappedComponent :type "PrimitiveComponent Object Reference") (OtherActor :type "Actor Object Reference") (OtherComp :type "PrimitiveComponent Object Reference") (OtherBodyIndex :type Integer))
  (bind _overlappingactors (`self.OverlappingActors`))
  (`KismetArrayLibrary.Array_RemoveItem` _overlappingactors OtherActor)
  (if (<= (`KismetArrayLibrary.Array_Length` _overlappingactors) 0)
    (set `self.bIsPressed` false)
    (`/Game/_Main/Blueprints/Object/BP_Door.CloseDoor` (`self.Door`))))

(fn `UserConstructionScript`)