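; BP_Door is a door actor that slides its Door component vertically between closed and open positions.
; BeginPlay stores the door's starting relative location as closed and sets the open position a fixed offset above it.
; OpenDoor and CloseDoor events play and reverse a timeline that lerps the door between those two positions.
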(event `OpenDoor`
  (bind (_direction _alpha) (`Timeline|DoorTimeline` :!label _label)
    (:`Update`
      (`SceneComponent.K2_SetRelativeLocation` (`self.Door`) (`KismetMathLibrary.VLerp` (`self.ClosedPosition`) (`self.OpenPosition`) _alpha) false false))))

(event `CloseDoor`
  (goto _label :!via `Reverse`))

(event `self.ReceiveBeginPlay`
  (bind _output_get (set `self.ClosedPosition` (`SceneComponent.RelativeLocation` (`self.Door`))))
  (set `self.OpenPosition` (+ _output_get (0.0 0.0 200.0))))

(fn `UserConstructionScript`)